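; RKTPawn_Blueprint is a pawn with an unfinished cable hook, built on a CableActor child actor.
; BeginPlay casts that child actor and hides its cable.
; Tick stores delta time and, while G is held with LastHook at zero, tests the cursor trace hit and its distance from the pawn.
; That test cannot pass (distance below zero) and triggers nothing, and the cable setup nodes are never executed.
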(event EventBeginPlay
  ;[1 1 1] Cable Initialize
  (bind _ascable_actor (Utilities|Casting|CastToCableActor (Variables|/Script/Engine.ChildActorComponent|GetChildActor (Variables|Default|GetCableActor))))
  (Rendering|SetVisibility (Variables|/Script/CableComponent.CableActor|GetCableComponent _ascable_actor) false false))

(event EventTick
  (params (DeltaSeconds :type Float%20%28single-precision%29))
  (bind _returnvalue (Game|GetPlayerController 0))
  (bind (_hitresult _returnvalue_2) (Game|Player|GetHitResultUnderCursorbyChannel _returnvalue "TraceTypeQuery1" true))
  (Variables|Default|SetDeltaTime DeltaSeconds)
  (if (and (Game|Player|IsInputKeyDown _returnvalue "G") (Math|Vector|Equal(Vector) (Variables|Default|GetLastHook) "0, 0, 0" 0.0001))
    (if (and (< (Math|Vector|VectorLength (- (Transformation|GetActorLocation) (.Location (Collision|BreakHitResult _hitresult)))) 0.0) _returnvalue_2)
      _)))

(fn ConstructionScript)