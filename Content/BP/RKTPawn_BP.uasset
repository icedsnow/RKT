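; Rocket pawn with a fireable grapple hook and pitch limiting near ceilings and ground.
; Fire launches a Grapple_BP from the left hook socket with inherited velocity; release destroys it.
; Tick updates the cable and, within slack range, constrains dynamic attachments to the capsule; static attachments get only zero-impulse placeholders.
; Nose traces up and down reset pitch limits, which Hit interpolates when they strike PhysicsVolumes; ground-slide and auto-break logic is unhooked.
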(event EventTick
  (params (DeltaSeconds :type Float%20%28single-precision%29))
  (Variables|Default|SetDeltaSeconds DeltaSeconds)
  (Utilities|FlowControl|Sequence
    (:then_0
      ;[1 1 1] Grapple
      (Utilities|IsValid (stale Input|ActionEvents|InputActionFire _returnvalue_4)
        (:Is%20Valid
          (Variables|/Game/BP/Grapple_BP.Grapple_BP_C|SetCableBase (stale Input|ActionEvents|InputActionFire _returnvalue_4) (+ (Transformation|GetSocketLocation (Variables|Default|GetRocketMesh) "RKT_L_Hook_Socket") "0, 0, 0"))
          (Default|CableLink (stale Input|ActionEvents|InputActionFire _returnvalue_4))
          ;;[0.05725 1 0] Fires up to here - Condition statement
          (if (< (Math|Vector|VectorLength (- (Transformation|GetActorLocation (stale Input|ActionEvents|InputActionFire _returnvalue_4)) (Transformation|GetActorLocation))) 1e+04)
            (Utilities|FlowControl|Gate true
              (:Exit
                ;;[1 0 0] False - Ready to Destroy cable
                (if (Variables|/Game/BP/Grapple_BP.Grapple_BP_C|GetAttachedToObject (stale Input|ActionEvents|InputActionFire _returnvalue_4))
                  ;;[1 1 1] True - (Attached to Object which is Dynamic*) Force update constrain, Impulse maybe
                  (if (Variables|/Game/BP/Grapple_BP.Grapple_BP_C|GetAttachedToDynamic (stale Input|ActionEvents|InputActionFire _returnvalue_4))
                    (if (Variables|/Game/BP/Grapple_BP.Grapple_BP_C|GetGrappleActive (stale Input|ActionEvents|InputActionFire _returnvalue_4))
                      ;;[1 0.9702 0] Attached to Dynamic Object
                      (Physics|AddImpulse (Variables|/Game/BP/Grapple_BP.Grapple_BP_C|GetCollisionComponent (stale Input|ActionEvents|InputActionFire _returnvalue_4)) "0, 0, 0" "None" false) ; Fires when grapple attaches to an object & > slack length
                      (Utilities|FlowControl|DoOnce false
                        (:Completed
                          (bind _returnvalue (AddComponent|AddPhysicsConstraintComponent (Components|GetOwner (Variables|/Game/BP/Grapple_BP.Grapple_BP_C|GetAttachedObject (stale Input|ActionEvents|InputActionFire _returnvalue_4))) false))
                          (Class|PhysicsConstraintComponent|SetConstrainedComponents _returnvalue (Variables|/Game/BP/Grapple_BP.Grapple_BP_C|GetAttachedObject (stale Input|ActionEvents|InputActionFire _returnvalue_4)) "None" (Variables|Default|GetCapsuleCollisionComponent) "None")
                          (bind _output_get (Variables|Default|SetConstraintActive true))
                          (if _output_get
                            (if (Variables|Default|GetConstraintActive)
                              (Utilities|FlowControl|Gate true) ; enters at Close
                              (else
                                (Utilities|FlowControl|Gate true) ; enters at Open
                              ))))))
                    (else
                      ;[0 1 0.4565] Attached to Static Object
                      (if (Variables|/Game/BP/Grapple_BP.Grapple_BP_C|GetGrappleAttachedToStatic (stale Input|ActionEvents|InputActionFire _returnvalue_4))
                        (Physics|AddImpulse (Variables|/Game/BP/Grapple_BP.Grapple_BP_C|GetCollisionComponent (stale Input|ActionEvents|InputActionFire _returnvalue_4)) "0, 0, 0" "None" false)
                        (Utilities|FlowControl|DoOnce false)))))))))))
    (:then_1
      ;[1 1 1] Supplies Tick
      (Utilities|FlowControl|Sequence
        (:then_1
          ;[1 1 1] Ceiling - Physics Volume
          (bind _outhit (Collision|LineTraceByChannel (+ (Transformation|GetSocketLocation (Variables|Default|GetRocketMesh) "RKT_Nose_Socket") "0, 0,90.000000") (+ (Transformation|GetSocketLocation (Variables|Default|GetRocketMesh) "RKT_Nose_Socket") (Math|Vector|MakeVector 0.0 0.0 1.3e+02)) "TraceTypeQuery1" false 0 "None" true "(R=1.000000,G=0.000000,B=0.000000,A=1.000000)" "(R=0.000000,G=1.000000,B=0.000000,A=1.000000)" 1.0))
          (bind _output_get_2 (Variables|Default|SetIsHittingCeiling (.bBlockingHit (Collision|BreakHitResult _outhit))))
          (if (not _output_get_2)
            (Variables|Default|SetMaxPitch 5.0)))
        (:then_2
          ;[1 1 1] Landscape
          (bind _outhit_2 (Collision|LineTraceByChannel (Transformation|GetSocketLocation (Variables|Default|GetRocketMesh) "RKT_Nose_Socket") (+ (Transformation|GetSocketLocation (Variables|Default|GetRocketMesh) "RKT_Nose_Socket") (Math|Vector|MakeVector 0.0 0.0 -2e+01)) "TraceTypeQuery1" false 0 "None" true "(R=1.000000,G=0.000000,B=0.000000,A=1.000000)" "(R=0.000000,G=1.000000,B=0.000000,A=1.000000)" 1.0))
          (Utilities|FlowControl|Sequence
            (:then_0
              ;[1 1 1] Temporary BP for appearance of sliding, Constrains Man/Min rotation
              (Variables|Default|SetIsHittingGround (.bBlockingHit (Collision|BreakHitResult _outhit_2)))
              (if (not false)
                (Variables|Default|SetMinPitch -5.0)))))))))

(event Collision|EventHit
  (params (MyComp :type Primitive%20Component%20Object%20Reference) (Other :type Actor%20Object%20Reference) (OtherComp :type Primitive%20Component%20Object%20Reference) (bSelfMoved :type Boolean) (HitLocation :type Vector :default "0, 0, 0") (HitNormal :type Vector :default "0, 0, 0") (NormalImpulse :type Vector :default "0, 0, 0") (Hit :type Hit%20Result%20Structure%20%28by%20ref%29))
  ;[1 1 1] Ceiling - Physics Volume
  (Utilities|FlowControl|Sequence
    (:then_0
      (if (Utilities|ClassIsChildOf (Utilities|GetClass (.HitActor (Collision|BreakHitResult (stale EventTick _outhit)))) "/Script/Engine.PhysicsVolume")
        (Variables|Default|SetMaxPitch (Math|Interpolation|FInterpTo (.Pitch (Math|Rotator|BreakRotator (Transformation|GetActorRotation))) -1.0 (Variables|Default|GetDeltaSeconds) 16.0))))
    (:then_1
      ;[1 1 1] Temporary BP for appearance of sliding, Constrains Man/Min rotation
      (if (Utilities|ClassIsChildOf (Utilities|GetClass (.HitActor (Collision|BreakHitResult (stale EventTick _outhit_2)))) "/Script/Engine.PhysicsVolume")
        (Variables|Default|SetMinPitch (Math|Interpolation|FInterpTo (.Pitch (Math|Rotator|BreakRotator (Transformation|GetActorRotation))) 1.0 (Variables|Default|GetDeltaSeconds) 16.0))))))

(event Input|ActionEvents|InputActionFire
  (params (Key :type Key%20Structure :default "AnyKey"))
  (bind _returnvalue (Math|Rotator|MakeRotator 0.0 0.0 -9e+01))
  (bind _returnvalue_2 (Transformation|GetActorRotation))
  (bind _returnvalue_3 (Math|Rotator|CombineRotators _returnvalue_2 _returnvalue))
  ;[1 1 1] Grapple
  (:Pressed
    (Utilities|FlowControl|DoOnce false :!label _label
      (:Completed
        (bind _returnvalue_4 (Game|SpawnActorfromClass "/Game/BP/Grapple_BP.Grapple_BP_C" (Math|Transform|MakeTransform (+ (Transformation|GetSocketLocation (Variables|Default|GetRocketMesh) "RKT_L_Hook_Socket") "0, 0, 0") _returnvalue_3) "AdjustIfPossibleButDontSpawnIfColliding" 0 "0.000000,0.000000,0.000000" true false false)) ; Spawn Projectile
        (bind _returnvalue_5 (Physics|GetPhysicsLinearVelocity (Variables|Default|GetCapsuleCollisionComponent) "None"))
        (Physics|AddImpulse (Variables|/Game/BP/Grapple_BP.Grapple_BP_C|GetCollisionComponent _returnvalue_4) (+ (* _returnvalue_5 1.0) (Math|Vector|RotateVector "5000.000000, 0, 0" _returnvalue_3)) "None" true)
        (Utilities|FlowControl|Gate true) ; enters at Open
      )))
  (:Released
    (Actor|DestroyActor _returnvalue_4)
    (Utilities|FlowControl|Sequence
      (:then_0
        (Utilities|FlowControl|Gate true) ; enters at Close
      )
      (:then_1
        ;;[1 0.9702 0] Attached to Dynamic Object
        (Variables|Default|SetConstraintActive false))
      (:then_2
        (goto _label_2 Toggle))
      (:then_3
        (Utilities|FlowControl|Gate true :!label _label_2
          (:Exit
            (Class|PhysicsConstraintComponent|BreakConstraint (stale EventTick _returnvalue))
            (Variables|Default|SetConstraintActive false))))
      (:then_4
        (goto _label Reset))
      (:then_5
        ;[0 1 0.4565] Attached to Static Object
        (Variables|Default|SetConstraintActive false)))))

(event Input|ActionEvents|InputActionFire
  (params (Key :type Key%20Structure :default "AnyKey"))
  ;[0 1 0.4565] Attached to Static Object
  (:Pressed
    (Utilities|FlowControl|DoOnce false) ; enters at Reset
  ))

(event Input|ActionEvents|InputActionFire
  (params (Key :type Key%20Structure :default "AnyKey"))
  ;[1 1 1] Grapple
  ;;[1 0.9702 0] Attached to Dynamic Object
  (:Pressed
    (Utilities|FlowControl|DoOnce false) ; enters at Reset
  ))

(fn ConstructionScript)