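; Grapple hook actor with a cable that latches onto whatever it hits.
; Hit sorts targets into non-player rockets, jockeys, physics bodies, landscape and static objects, setting attachment flags and attaching to all but landscape.
; Static hits disable sphere collision and gravity and toggle a Tick gate that pins the hook to the impact point.
; Cable placement uses CableBase; jockey self-checks and server hit handling are unfinished.
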(event Custom|ServerAttemptsHit
  ;[0 1 0.187] Server Executes Hit
  (Networking|SwitchHasAuthority))

(event EventTick
  (params (DeltaSeconds :type Float%20%28single-precision%29))
  (Utilities|FlowControl|Sequence
    (:then_0
      (Utilities|FlowControl|Gate true
        (:Exit
          (Transformation|SetActorLocation (.ImpactPoint (Collision|BreakHitResult (stale Collision|EventHit Hit))) true true))))))

(event Collision|EventHit
  (params (MyComp :type Primitive%20Component%20Object%20Reference) (Other :type Actor%20Object%20Reference) (OtherComp :type Primitive%20Component%20Object%20Reference) (bSelfMoved :type Boolean) (HitLocation :type Vector :default "0, 0, 0") (HitNormal :type Vector :default "0, 0, 0") (NormalImpulse :type Vector :default "0, 0, 0") (Hit :type Hit%20Result%20Structure%20%28by%20ref%29))
  (bind _returnvalue (Utilities|GetClass Other))
  (bind (_bblockinghit _binitialoverlap _time _location _impactpoint _normal _impactnormal _physmat _hitactor) (Collision|BreakHitResult Hit))
  (if (not (Utilities|ClassIsChildOf _returnvalue "Grapple_BP_C"))
    (if (not (Utilities|ClassIsChildOf _returnvalue "/Script/Engine.PhysicsVolume"))
      ;[1 1 1] This needs to change with Grapple -> Rocket Implementation
      (if (Utilities|ClassIsChildOf _returnvalue "/Game/BP/Rockets/RKTPawn_BP.RKTPawn_BP_C")
        ;[1 0 0] Check for Rocket self VS Enemy Rocket
        (if (not (Pawn|IsPlayerControlled (Variables|/Script/Engine.Actor|GetInstigator Other)))
          (Development|PrintString "Hit Enemy Rocket")
          (Variables|Default|SetAttachedToRKT true)
          (Variables|Default|SetAttachedToObject true)
          (Transformation|AttachActorToActor Other "None" "KeepWorld" "KeepWorld" "KeepWorld" true)
          (bind _output_get (Variables|Default|SetAttachedObject OtherComp))
          (Class|PrimitiveComponent|WakeRigidBody _output_get "None")
          (Variables|Default|SetAttachedObjectActor Other))
        (else
          (Utilities|FlowControl|Sequence
            (:then_0
              (Variables|Default|SetAttachedToObject true)
              (if (Utilities|ClassIsChildOf _returnvalue "/Game/BP/Characters/RKT_Jockey_BP.RKT_Jockey_BP_C")
                ;[1 1 1] Check for Self vs Enemy Jockey - NYI
                (if true
                  (Variables|Default|SetAttachedToJockey true)
                  (Transformation|AttachActorToActor Other "None" "KeepWorld" "KeepWorld" "KeepWorld" true)
                  (bind _output_get_2 (Variables|Default|SetAttachedObject OtherComp))
                  (Class|PrimitiveComponent|WakeRigidBody OtherComp "None")
                  (Variables|Default|SetAttachedObjectActor Other)
                  (Physics|SetEnableGravity _output_get_2 true))
                (elif (Physics|IsSimulatingPhysics OtherComp "None")
                  (Utilities|FlowControl|DoOnce false
                    (:Completed
                      (Transformation|AttachActorToActor Other "None" "KeepWorld" "KeepWorld" "KeepWorld" true)
                      (Variables|Default|SetAttachedObject OtherComp)
                      (Variables|Default|SetAttachedToDynamic true)
                      (Class|PrimitiveComponent|WakeRigidBody OtherComp "None")
                      (Variables|Default|SetAttachedObjectActor Other)))
                  (elif (not (Variables|Default|GetAttachedToDynamic))
                    (if (Utilities|ClassIsChildOf (Utilities|GetClass _hitactor) "/Script/Landscape.Landscape")
                      (Variables|Default|SetAttachedToLandscape true)
                      (else
                        (Utilities|FlowControl|DoOnce false
                          (:Completed
                            (Transformation|AttachActorToActor Other "None" "KeepWorld" "KeepWorld" "KeepWorld" true)
                            (Variables|Default|SetAttachedStatic OtherComp)
                            (Variables|Default|SetAttachedStaticActor Other)
                            (Variables|Default|SetAttachedToStatic true)
                            (Collision|SetCollisionEnabled (Variables|Default|GetSphere) "NoCollision")
                            (Physics|SetEnableGravity (Variables|Default|GetCollisionComponent) false)
                            (Utilities|FlowControl|Gate true) ; enters at Toggle
                          ))))))))
            (:then_2
              ;[1 1 1] Print
              (Utilities|FlowControl|DoOnce false
                (:Completed
                  (Development|PrintString "Grapple HIT:")
                  (Development|PrintString (Utilities|GetDisplayName _hitactor)))))
            (:then_3
              ;[1 1 1] Not Sure Used
              (Variables|Default|SetGameTimeSinceSpawned (Actor|GetGameTimeSinceCreation)))))))))

(fn ConstructionScript
  (Transformation|SetRelativeLocation (Variables|Default|GetCable1) (Variables|Default|GetCableBase) false false))

(fn CableLink
  (Transformation|SetWorldLocation (Variables|Default|GetCable1) (Variables|Default|GetCableBase) false false))