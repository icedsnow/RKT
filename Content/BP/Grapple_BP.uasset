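; Grapple hook projectile with a cable that sticks to what it hits, ignoring other grapples and RKTPawn_BP.
; On hit it attaches to the actor, recording the component and waking it if physics-simulated, or flagging it as static otherwise.
; Static hits also disable sphere collision and gravity and toggle a Tick gate that pins the hook to the impact point.
; CableLink and the construction script position the cable at CableBase.
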(event EventTick
  (params (DeltaSeconds :type Float%20%28single-precision%29))
  (Utilities|FlowControl|Sequence
    (:then_0
      (Utilities|FlowControl|Gate true
        (:Exit
          (Transformation|SetActorLocation (.ImpactPoint (Collision|BreakHitResult (stale Collision|EventHit Hit))) false false))))))

(event Collision|EventHit
  (params (MyComp :type Primitive%20Component%20Object%20Reference) (Other :type Actor%20Object%20Reference) (OtherComp :type Primitive%20Component%20Object%20Reference) (bSelfMoved :type Boolean) (HitLocation :type Vector :default "0, 0, 0") (HitNormal :type Vector :default "0, 0, 0") (NormalImpulse :type Vector :default "0, 0, 0") (Hit :type Hit%20Result%20Structure%20%28by%20ref%29))
  (bind (_bblockinghit _binitialoverlap _time _location _impactpoint _normal _impactnormal _physmat _hitactor) (Collision|BreakHitResult Hit))
  (bind _returnvalue (Utilities|GetClass Other))
  (if (not (Utilities|ClassIsChildOf _returnvalue "Grapple_BP_C"))
    (if (not (Utilities|ClassIsChildOf _returnvalue "/Game/BP/RKTPawn_BP.RKTPawn_BP_C"))
      (Utilities|FlowControl|Sequence
        (:then_0
          (if (Physics|IsSimulatingPhysics OtherComp "None")
            (Utilities|FlowControl|DoOnce false
              (:Completed
                (Transformation|AttachActorToActor Other "None" "KeepWorld" "KeepWorld" "KeepWorld" true)
                (Variables|Default|SetAttachedObject OtherComp)
                (Variables|Default|SetAttachedToDynamic true)
                (Class|PrimitiveComponent|WakeRigidBody OtherComp "None")
                (Variables|Default|SetAttachedObjectActor Other)))
            (elif (not (Variables|Default|GetAttachedToDynamic))
              (Utilities|FlowControl|DoOnce false
                (:Completed
                  (Transformation|AttachActorToActor Other "None" "KeepWorld" "KeepWorld" "KeepWorld" true)
                  (Variables|Default|SetAttachedToStatic true)
                  (Collision|SetCollisionEnabled (Variables|Default|GetSphere) "NoCollision")
                  (Physics|SetEnableGravity (Variables|Default|GetCollisionComponent) false)
                  (Utilities|FlowControl|Gate true) ; enters at Toggle
                )))))
        (:then_1
          (Utilities|FlowControl|DoOnce false
            (:Completed
              (Development|PrintString (Utilities|GetDisplayName _hitactor)))))
        (:then_2
          (Variables|Default|SetAttachedToObject true))
        (:then_3
          (Variables|Default|SetGameTimeSinceSpawned (Actor|GetGameTimeSinceCreation)))))))

(fn ConstructionScript
  (Transformation|SetRelativeLocation (Variables|Default|GetCable1) (Variables|Default|GetCableBase) false false))

(fn CableLink
  (Transformation|SetWorldLocation (Variables|Default|GetCable1) (Variables|Default|GetCableBase) false false))