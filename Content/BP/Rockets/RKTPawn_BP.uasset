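; Rocket pawn that fires left and right Grapple_BP hooks to tether itself to other objects.
; Fire inputs launch hooks with inherited velocity; Tick updates cables, line-traces paths and destroys hooks on overstretch or missed attachment.
; The left hook uses elastic, mass-scaled impulses for movable targets and constraints for static ones, while the right uses constraints for both.
; Hit redirects off walls and poles, with physics toggling as a recurring bug workaround.
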(event Collision|EventHit
  (params (MyComp :type Primitive%20Component%20Object%20Reference) (Other :type Actor%20Object%20Reference) (OtherComp :type Primitive%20Component%20Object%20Reference) (bSelfMoved :type Boolean) (HitLocation :type Vector :default "0, 0, 0") (HitNormal :type Vector :default "0, 0, 0") (NormalImpulse :type Vector) (Hit :type Hit%20Result%20Structure%20%28by%20ref%29))
  (bind (_bblockinghit _binitialoverlap _time _location _impactpoint _normal _impactnormal _physmat _hitactor _hitcomponent) (Collision|BreakHitResult Hit))
  (bind _rocketmesh_ref (Variables|Default|GetRocketMesh_Ref))
  (bind _rocketmesh_ref_2 (Variables|Default|GetRocketMesh_Ref))
  (bind _returnvalue (Utilities|GetClass _hitactor))
  ;[0.9167 1 0] Event Hit
  (Utilities|FlowControl|Sequence
    (:then_0
      ;[0.04649 1 0] LANDSCAPE - COLLISION LINETRACE - SET PITCH TO ZERO
      ;;[1 1 1] Temp - Only use for Ceiling Physics Volume, Ignore Actor breaks physics everywhere else --- Thoroughly Tested
      (if (Utilities|ClassIsChildOf _returnvalue "/Script/Engine.PhysicsVolume")
        (Collision|IgnoreActorwhenMoving (Variables|Default|GetRocketMesh_Ref) _hitactor true)))
    (:then_1
      ;[0 0.9936 1] WALL BP - COLLISION HANDLING
      (if (Utilities|ClassIsChildOf (Utilities|GetClass _hitactor) "/Game/BP/LevelAssets/Temp_Wall_BP.Temp_Wall_BP_C")
        (Transformation|SetActorRotation (Math|Conversions|RotationFromXVector (Math|Vector|RotateVector _impactnormal "0.000000,15.000000, 0")) true)
        (Utilities|FlowControl|Sequence
          (:then_0
            ;;[1 0.004134 0] Fixes most physics bugs after break
            (Class|PrimitiveComponent|SetAllPhysicsLinearVelocity _rocketmesh_ref "0, 0, 0" false :!label _label)
            (Physics|SetSimulatePhysics _rocketmesh_ref false)
            (Utilities|FlowControl|Delay 0.1)
            (Class|PrimitiveComponent|SetAllPhysicsLinearVelocity _rocketmesh_ref "0, 0, 0" false)
            (Physics|SetSimulatePhysics _rocketmesh_ref true)
            (Utilities|FlowControl|DoN 5 :!label _label_2
              (:Exit
                (goto _label)))))
        (else
          ;[1 0.4611 0] CheckerPole BP Collision
          (if (Utilities|ClassIsChildOf _returnvalue "/Game/BP/LevelAssets/CheckerPole_Blueprint.CheckerPole_Blueprint_C")
            (Transformation|SetActorRotation (Math|Conversions|RotationFromXVector (Math|Vector|RotateVector _impactnormal "0.000000,220.000000, 0")) true)
            ;[1 0 0.004658] Temp Physics Bug Fix
            (Class|PrimitiveComponent|SetAllPhysicsLinearVelocity _rocketmesh_ref_2 "0, 0, 0" false)
            (Physics|SetSimulatePhysics _rocketmesh_ref_2 false)
            (Class|PrimitiveComponent|SetAllPhysicsLinearVelocity _rocketmesh_ref_2 "0, 0, 0" false)
            (Physics|SetSimulatePhysics _rocketmesh_ref_2 true)))))
    (:then_2
      (goto _label_2 Reset))
    (:then_3
      ;[1 0.9702 0] Attached to Dynamic Object
      (if (== _hitcomponent (Variables|/Game/BP/Gameplay/Grapple_BP.Grapple_BP_C|GetAttachedObject (stale Input|ActionEvents|InputActionFire _returnvalue_6)))
        _))))

(event EventTick
  (params (DeltaSeconds :type Float%20%28single-precision%29))
  (bind _returnvalue (Math|Rotator|MakeRotator 0.0 0.0 9e+01))
  (bind _returnvalue_2 (Math|Rotator|MakeRotator 0.0 0.0 -9e+01))
  (bind _returnvalue_3 (Transformation|GetActorRotation))
  (bind _returnvalue_4 (Transformation|GetActorRotation))
  (bind _returnvalue_5 (Transformation|GetActorLocation))
  (bind _returnvalue_6 (Transformation|GetActorRotation))
  (bind _rocketmesh_ref (Variables|Default|GetRocketMesh_Ref))
  (bind _rocketmesh (Variables|Default|GetRocketMesh))
  (bind _rocketmesh_2 (Variables|Default|GetRocketMesh))
  (bind _rocketmesh_ref_2 (Variables|Default|GetRocketMesh_Ref))
  (bind _rocketmesh_ref_3 (Variables|Default|GetRocketMesh_Ref))
  (bind _rocketmesh_ref_4 (Variables|Default|GetRocketMesh_Ref))
  (bind _rocketmesh_ref_5 (Variables|Default|GetRocketMesh_Ref))
  (bind _rocketmesh_ref_6 (Variables|Default|GetRocketMesh_Ref))
  (bind _rocketmesh_ref_7 (Variables|Default|GetRocketMesh_Ref))
  (bind _returnvalue_7 (Math|Rotator|CombineRotators _returnvalue_3 _returnvalue_2))
  (bind _returnvalue_8 (Transformation|GetSocketLocation _rocketmesh "RKT_L_Hook_Socket"))
  (bind _returnvalue_9 (Math|Rotator|CombineRotators _returnvalue_4 _returnvalue))
  (bind _returnvalue_10 (Transformation|GetSocketLocation _rocketmesh_ref_3 "RKT_R_Hook_Socket"))
  (bind (_roll _pitch _yaw) (Math|Rotator|BreakRotator _returnvalue_6))
  (bind _returnvalue_11 (+ _returnvalue_10 "0, 0, 0"))
  (bind _returnvalue_12 (+ _returnvalue_8 "0, 0, 0"))
  ;[0.145 0.1826 0.225] Tick Sequence
  (Variables|Default|SetDeltaSeconds DeltaSeconds)
  (Utilities|FlowControl|Sequence
    (:then_0
      (Utilities|IsValid (stale Input|ActionEvents|InputActionFire _returnvalue_6)
        (:Is%20Valid
          (Variables|/Game/BP/Gameplay/Grapple_BP.Grapple_BP_C|SetCableBase (stale Input|ActionEvents|InputActionFire _returnvalue_6) _returnvalue_12)
          (Default|CableLink (stale Input|ActionEvents|InputActionFire _returnvalue_6))
          ;[0.05725 1 0] Tick Fires up to here - Condition statement
          (if true
            (Utilities|FlowControl|Sequence
              (:then_0
                (Utilities|FlowControl|Gate true :!label _label
                  (:Exit
                    (Utilities|FlowControl|Sequence
                      (:then_0
                        (if (Variables|/Game/BP/Gameplay/Grapple_BP.Grapple_BP_C|GetAttachedToRKT (stale Input|ActionEvents|InputActionFire _returnvalue_6))
                          (if true
                            ;[0.73 0.1108 0] Attached To Rocket
                            (if (> (Variables|Default|GetCableSlackLength) 5e+02)
                              (Physics|AddImpulse (Variables|/Game/BP/Gameplay/Grapple_BP.Grapple_BP_C|GetAttachedObject (stale Input|ActionEvents|InputActionFire _returnvalue_6)) (* (* (* (Variables|Default|GetVelocityRKT) (Math|Float|Sqrt (Variables|Default|GetCableSlackLength))) 0.0033) (* (/ (Physics|GetMass (Variables|/Game/BP/Gameplay/Grapple_BP.Grapple_BP_C|GetAttachedObject (stale Input|ActionEvents|InputActionFire _returnvalue_6))) (Physics|GetMass (Variables|Default|GetRocketMesh_Ref))) -1.0)) "None" true)
                              (Class|PrimitiveComponent|SetLinearDamping (Variables|/Game/BP/Gameplay/Grapple_BP.Grapple_BP_C|GetAttachedObject (stale Input|ActionEvents|InputActionFire _returnvalue_6)) 2.0)
                              (Class|PrimitiveComponent|SetAngularDamping (Variables|/Game/BP/Gameplay/Grapple_BP.Grapple_BP_C|GetAttachedObject (stale Input|ActionEvents|InputActionFire _returnvalue_6)) 1.0)
                              (if (> (Variables|Default|GetCableSlackLength) 8e+02)
                                (Physics|AddImpulse _rocketmesh_ref (* (* (* (* (Variables|Default|GetVelocityRKT) (Math|Float|Sqrt (Variables|Default|GetCableSlackLength))) 0.0033) (* (/ (Physics|GetMass (Variables|/Game/BP/Gameplay/Grapple_BP.Grapple_BP_C|GetAttachedObject (stale Input|ActionEvents|InputActionFire _returnvalue_6))) (Physics|GetMass (Variables|Default|GetRocketMesh_Ref))) -1.0)) -0.5) "None" true)
                                (Class|PrimitiveComponent|SetLinearDamping _rocketmesh_ref 2.0)
                                (Class|PrimitiveComponent|SetAngularDamping _rocketmesh_ref 1e+01))))
                          (elif (Variables|/Game/BP/Gameplay/Grapple_BP.Grapple_BP_C|GetAttachedToObject (stale Input|ActionEvents|InputActionFire _returnvalue_6))
                            (if (Variables|/Game/BP/Gameplay/Grapple_BP.Grapple_BP_C|GetAttachedToJockey (stale Input|ActionEvents|InputActionFire _returnvalue_6))
                              ;[0.3525 1 0] Attached To Jockey
                              (if true
                                (if (> (Variables|Default|GetCableSlackLength) 3e+02)
                                  (Physics|AddImpulse (Variables|/Game/BP/Gameplay/Grapple_BP.Grapple_BP_C|GetAttachedObject (stale Input|ActionEvents|InputActionFire _returnvalue_6)) (* (* (* (Variables|Default|GetVelocityRKT) (Math|Float|Sqrt (Variables|Default|GetCableSlackLength))) 0.1) (* (/ (Physics|GetMass (Variables|/Game/BP/Gameplay/Grapple_BP.Grapple_BP_C|GetAttachedObject (stale Input|ActionEvents|InputActionFire _returnvalue_6))) (Physics|GetMass (Variables|Default|GetRocketMesh_Ref))) -1.0)) "None" true)
                                  (Class|PrimitiveComponent|SetLinearDamping (Variables|/Game/BP/Gameplay/Grapple_BP.Grapple_BP_C|GetAttachedObject (stale Input|ActionEvents|InputActionFire _returnvalue_6)) 18.0)
                                  (Class|PrimitiveComponent|SetAngularDamping (Variables|/Game/BP/Gameplay/Grapple_BP.Grapple_BP_C|GetAttachedObject (stale Input|ActionEvents|InputActionFire _returnvalue_6)) 0.3)
                                  (Class|PrimitiveComponent|SetLinearDamping _rocketmesh_ref_7 1e+06)
                                  (Class|PrimitiveComponent|SetAngularDamping _rocketmesh_ref_7 1e+06)))
                              (elif (Variables|/Game/BP/Gameplay/Grapple_BP.Grapple_BP_C|GetAttachedToDynamic (stale Input|ActionEvents|InputActionFire _returnvalue_6))
                                (if (Variables|/Game/BP/Gameplay/Grapple_BP.Grapple_BP_C|GetGrappleActive (stale Input|ActionEvents|InputActionFire _returnvalue_6))
                                  ;[1 0.9702 0] Attached to Dynamic Object
                                  (Physics|AddImpulse (Variables|/Game/BP/Gameplay/Grapple_BP.Grapple_BP_C|GetCollisionComponent (stale Input|ActionEvents|InputActionFire _returnvalue_6)) "0, 0, 0" "None" false) ; Fires when grapple attaches to an object & > slack length
                                  (if (not (Utilities|ClassIsChildOf (Utilities|GetClass (.HitComponent (Collision|BreakHitResult (stale _outhit)))) "RKTPawn_BP_C"))
                                    (Utilities|IsValid (Variables|/Game/BP/Gameplay/Grapple_BP.Grapple_BP_C|GetAttachedObject (stale Input|ActionEvents|InputActionFire _returnvalue_6))
                                      (:Is%20Valid
                                        (if (> (Variables|Default|GetCableSlackLength) 3e+02)
                                          (Utilities|FlowControl|Sequence
                                            (:then_0
                                              (Physics|AddImpulse (Variables|/Game/BP/Gameplay/Grapple_BP.Grapple_BP_C|GetAttachedObject (stale Input|ActionEvents|InputActionFire _returnvalue_6)) (* (* (* (Variables|Default|GetVelocityRKT) (Math|Float|Sqrt (Variables|Default|GetCableSlackLength))) 2.0) (* (/ (Physics|GetMass (Variables|/Game/BP/Gameplay/Grapple_BP.Grapple_BP_C|GetAttachedObject (stale Input|ActionEvents|InputActionFire _returnvalue_6))) (Physics|GetMass (Variables|Default|GetRocketMesh_Ref))) -1.0)) "None" false)
                                              (Class|PrimitiveComponent|SetLinearDamping (Variables|/Game/BP/Gameplay/Grapple_BP.Grapple_BP_C|GetAttachedObject (stale Input|ActionEvents|InputActionFire _returnvalue_6)) 0.25)
                                              (Class|PrimitiveComponent|SetAngularDamping (Variables|/Game/BP/Gameplay/Grapple_BP.Grapple_BP_C|GetAttachedObject (stale Input|ActionEvents|InputActionFire _returnvalue_6)) 0.0)
                                              (Class|PrimitiveComponent|SetLinearDamping _rocketmesh_ref_5 1e+06)
                                              (Class|PrimitiveComponent|SetAngularDamping _rocketmesh_ref_5 1e+06))))))))
                                (else
                                  ;[1 1 1] Static
                                  (if (Variables|/Game/BP/Gameplay/Grapple_BP.Grapple_BP_C|GetAttachedToStatic (stale Input|ActionEvents|InputActionFire _returnvalue_6))
                                    ;[0 1 0.4565] Attached to Static Object
                                    (if true
                                      (if (not (Utilities|ClassIsChildOf (Utilities|GetClass (.HitComponent (Collision|BreakHitResult (stale _outhit)))) "RKTPawn_BP_C"))
                                        (Utilities|IsValid (Variables|/Game/BP/Gameplay/Grapple_BP.Grapple_BP_C|GetAttachedStatic (stale Input|ActionEvents|InputActionFire _returnvalue_6))
                                          (:Is%20Valid
                                            (if (not (Utilities|ClassIsChildOf (Utilities|GetClass (.HitComponent (Collision|BreakHitResult (stale _outhit)))) "/Script/Landscape.Landscape"))
                                              (Utilities|FlowControl|Sequence
                                                (:then_0
                                                  (Utilities|FlowControl|DoOnce false :!label _label_2
                                                    (:Completed
                                                      (bind _returnvalue_13 (AddComponent|AddPhysicsConstraintComponent (Variables|/Game/BP/Gameplay/Grapple_BP.Grapple_BP_C|GetAttachedStaticActor (stale Input|ActionEvents|InputActionFire _returnvalue_6)) false))
                                                      (Class|PhysicsConstraintComponent|SetConstrainedComponents _returnvalue_13 (Variables|/Game/BP/Gameplay/Grapple_BP.Grapple_BP_C|GetAttachedStatic (stale Input|ActionEvents|InputActionFire _returnvalue_6)) "None" (Variables|/Game/BP/Gameplay/Grapple_BP.Grapple_BP_C|GetCollisionComponent (stale Input|ActionEvents|InputActionFire _returnvalue_6)) "None")
                                                      (bind _returnvalue_14 (AddComponent|AddPhysicsConstraintComponent (stale Input|ActionEvents|InputActionFire _returnvalue_6) false))
                                                      (Class|PhysicsConstraintComponent|SetConstrainedComponents _returnvalue_14 (Variables|/Game/BP/Gameplay/Grapple_BP.Grapple_BP_C|GetCollisionComponent (stale Input|ActionEvents|InputActionFire _returnvalue_6)) "None" (Variables|Default|GetRocketMesh) "None")
                                                      (if true
                                                        (goto _label_5 Open)))))
                                                (:then_1
                                                  (Utilities|IsValid _returnvalue_13
                                                    (:Is%20Valid
                                                      (Utilities|IsValid (Variables|/Game/BP/Gameplay/Grapple_BP.Grapple_BP_C|GetAttachedStatic (stale Input|ActionEvents|InputActionFire _returnvalue_6))
                                                        (:Is%20Not%20Valid
                                                          (goto _label_5 Close)))))))))))))))))))
                      (:then_1
                        ;[0.6243 0.7252 1] Line Trace to detect hits along grapple route
                        (bind (_outhit _returnvalue_15) (Collision|LineTraceByChannel _returnvalue_12 (Transformation|GetWorldLocation (Variables|/Game/BP/Gameplay/Grapple_BP.Grapple_BP_C|GetSphere (stale Input|ActionEvents|InputActionFire _returnvalue_6))) "TraceTypeQuery1" false (Utilities|Array|MakeArray (stale Input|ActionEvents|InputActionFire _returnvalue_6) (Variables|/Game/BP/Gameplay/Grapple_BP.Grapple_BP_C|GetAttachedObjectActor (stale Input|ActionEvents|InputActionFire _returnvalue_6)) (Variables|/Game/BP/Gameplay/Grapple_BP.Grapple_BP_C|GetAttachedStaticActor (stale Input|ActionEvents|InputActionFire _returnvalue_6))) "None"))
                        (if _returnvalue_15
                          (if (not (Variables|/Game/BP/Gameplay/Grapple_BP.Grapple_BP_C|GetAttachedToObject (stale Input|ActionEvents|InputActionFire _returnvalue_6)))
                            (Utilities|FlowControl|DoOnce false :!label _label_3
                              (:Completed
                                (Transformation|SetActorLocation (stale Input|ActionEvents|InputActionFire _returnvalue_6) (.ImpactPoint (Collision|BreakHitResult _outhit)) false false)
                                (goto _label))))))))))
              (:then_1
                ;[0 0 0] Conditional Destroy Actor Spaghetti
                (Variables|Default|SetCableSlackLength (Math|Vector|VectorLength (- (Transformation|GetActorLocation (stale Input|ActionEvents|InputActionFire _returnvalue_6)) (Transformation|GetActorLocation))))
                (Variables|Default|SetVelocityRKT (- (Transformation|GetActorLocation (stale Input|ActionEvents|InputActionFire _returnvalue_6)) (Transformation|GetActorLocation)))
                (if (Variables|/Game/BP/Gameplay/Grapple_BP.Grapple_BP_C|GetAttachedToObject (stale Input|ActionEvents|InputActionFire _returnvalue_6))
                  (if (> (Variables|Default|GetCableSlackLength) 2.2e+03)
                    (Utilities|IsValid (stale Input|ActionEvents|InputActionFire _returnvalue_6) :!label _label_4
                      (:Is%20Valid
                        _)
                      (:Is%20Not%20Valid
                        _))
                    (Actor|DestroyActor (stale Input|ActionEvents|InputActionFire _returnvalue_6))
                    (Utilities|FlowControl|Sequence
                      (:then_0
                        (goto _label Close))
                      (:then_2
                        (Utilities|FlowControl|Gate true :!label _label_5
                          (:Exit
                            (Class|PhysicsConstraintComponent|BreakConstraint _returnvalue_13)
                            (Class|PhysicsConstraintComponent|BreakConstraint _returnvalue_14)
                            (Utilities|FlowControl|Sequence
                              (:then_0
                                (goto _label_2 Reset))
                              (:then_1
                                ;[1 0.004134 0] Fixes most constraint physics bugs after break
                                (Class|PrimitiveComponent|SetAllPhysicsLinearVelocity _rocketmesh_ref_2 "0, 0, 0" false)
                                (Physics|SetSimulatePhysics _rocketmesh_ref_2 false)
                                (Physics|SetSimulatePhysics _rocketmesh_ref_2 true))))))
                      (:then_4
                        (Utilities|FlowControl|DoOnce false) ; enters at Reset
                      )
                      (:then_5
                        ;;[1 1 1] Connects from Destroy Spaghetti
                        (if true
                          (goto _label_3 Reset)))
                      (:then_6
                        (Variables|Default|SetGrappleReleased true)
                        (if (Variables|Default|GetGrappleReleased)
                          (Utilities|FlowControl|Sequence
                            (:then_0
                              ;[1 0.004134 0] Fixes most constraint physics bugs after break
                              (Class|PrimitiveComponent|SetAllPhysicsLinearVelocity _rocketmesh_ref_4 "0, 0, 0" false)
                              (Physics|SetSimulatePhysics _rocketmesh_ref_4 false)
                              (Physics|SetSimulatePhysics _rocketmesh_ref_4 true)))))
                      (:then_7
                        (Class|PrimitiveComponent|SetAngularDamping _rocketmesh_ref_6 0.0)
                        (Class|PrimitiveComponent|SetLinearDamping _rocketmesh_ref_6 0.01)
                        (Class|PrimitiveComponent|SetAngularDamping (Variables|/Game/BP/Gameplay/Grapple_BP.Grapple_BP_C|GetAttachedObject (stale Input|ActionEvents|InputActionFire _returnvalue_6)) 0.0)
                        (Class|PrimitiveComponent|SetLinearDamping (Variables|/Game/BP/Gameplay/Grapple_BP.Grapple_BP_C|GetAttachedObject (stale Input|ActionEvents|InputActionFire _returnvalue_6)) 0.01))))
                  (else
                    (Utilities|FlowControl|Delay 1.0)
                    (if (not (Variables|/Game/BP/Gameplay/Grapple_BP.Grapple_BP_C|GetAttachedToObject (stale Input|ActionEvents|InputActionFire _returnvalue_6)))
                      (goto _label_4)))))
              (:then_2
                (Variables|Default|SetGrappleReleased false)))))))
    (:then_1
      ;[0.2318 1 0] Supplies Tick
      (Utilities|FlowControl|Sequence
        (:then_1
          ;[0.04649 1 0] LANDSCAPE - COLLISION LINETRACE - SET PITCH TO ZERO
          (bind (_outhit_2 _returnvalue_16) (Collision|LineTraceByChannel (+ _returnvalue_5 "0.000000,0.000000,-50.000000") (+ _returnvalue_5 "0.000000,0.000000,-100.000000") "TraceTypeQuery1" false 0 "None" true "(R=1.000000,G=0.000000,B=0.000000,A=1.000000)" "(R=0.000000,G=1.000000,B=0.000000,A=1.000000)" 1.0))
          (if _returnvalue_16
            (if (Utilities|ClassIsChildOf (Utilities|GetClass (.HitActor (Collision|BreakHitResult (stale Collision|EventHit Hit)))) "/Script/Landscape.Landscape")
              (if (<= (Variables|Default|GetMoveUpAxisValue) 0.0)
                (Transformation|SetActorRotation (Math|Rotator|MakeRotator _roll 0.0 _yaw) true)
                (Variables|Default|SetMinPitch 0.0)))
            (else
              (Variables|Default|SetMinPitch -5.0))))
        (:then_3
          ;[1 0 0.7247] Temporary Workaround - DO NOT USE
          (if (stale _output_get_2)
            ;;[1 1 1] Tick
            (if (not (Variables|/Game/BP/Gameplay/Grapple_BP.Grapple_BP_C|GetGrappleActive (stale Input|ActionEvents|InputActionRightFire _returnvalue_6)))
              (Collision|SetCollisionObjectType (stale _output_get) "ECC_PhysicsBody")
              (Variables|Default|SetBallIgnored_Alt false)
              ;[0 0.01606 1] Alt Fire
              ;;[1 0.004134 0] Fixes most constraint physics bugs after break
              (Class|PrimitiveComponent|SetAllPhysicsLinearVelocity _rocketmesh_2 "0, 0, 0" false :!label _label_6)
              (Physics|SetSimulatePhysics _rocketmesh_2 false)
              (Physics|SetSimulatePhysics _rocketmesh_2 true))))))
    (:then_2
      ;;[0.145 0.1826 0.225] Tick Sequence
      (Utilities|FlowControl|Sequence
        (:then_0
          (Utilities|IsValid (stale Input|ActionEvents|InputActionRightFire _returnvalue_6)
            (:Is%20Valid
              (Variables|/Game/BP/Gameplay/Grapple_BP.Grapple_BP_C|SetCableBase (stale Input|ActionEvents|InputActionRightFire _returnvalue_6) _returnvalue_11)
              (Default|CableLink (stale Input|ActionEvents|InputActionRightFire _returnvalue_6))
              ;;[0.05725 1 0] Tick Fires up to here - Condition statement
              (if true
                (Utilities|FlowControl|Sequence
                  (:then_0
                    (Utilities|FlowControl|Gate true :!label _label_7
                      (:Exit
                        (Utilities|FlowControl|Sequence
                          (:then_0
                            (if (Variables|/Game/BP/Gameplay/Grapple_BP.Grapple_BP_C|GetAttachedToObject (stale Input|ActionEvents|InputActionRightFire _returnvalue_6))
                              (if (Variables|/Game/BP/Gameplay/Grapple_BP.Grapple_BP_C|GetAttachedToDynamic (stale Input|ActionEvents|InputActionRightFire _returnvalue_6))
                                (if (Variables|/Game/BP/Gameplay/Grapple_BP.Grapple_BP_C|GetGrappleActive (stale Input|ActionEvents|InputActionRightFire _returnvalue_6))
                                  ;;[1 0.9702 0] Attached to Dynamic Object
                                  (Physics|AddImpulse (Variables|/Game/BP/Gameplay/Grapple_BP.Grapple_BP_C|GetCollisionComponent (stale Input|ActionEvents|InputActionRightFire _returnvalue_6)) "0, 0, 0" "None" false) ; Fires when grapple attaches to an object & > slack length
                                  (if (not (Utilities|ClassIsChildOf (Utilities|GetClass (.HitComponent (Collision|BreakHitResult (stale _outhit_3)))) "RKTPawn_BP_C"))
                                    (Utilities|IsValid (Variables|/Game/BP/Gameplay/Grapple_BP.Grapple_BP_C|GetAttachedObject (stale Input|ActionEvents|InputActionRightFire _returnvalue_6))
                                      (:Is%20Valid
                                        (Utilities|FlowControl|Sequence
                                          (:then_0
                                            (Utilities|FlowControl|DoOnce false :!label _label_8
                                              (:Completed
                                                (bind _returnvalue_17 (AddComponent|AddPhysicsConstraintComponent (Variables|/Game/BP/Gameplay/Grapple_BP.Grapple_BP_C|GetAttachedObjectActor (stale Input|ActionEvents|InputActionRightFire _returnvalue_6)) false))
                                                (Class|PhysicsConstraintComponent|SetConstrainedComponents _returnvalue_17 (Variables|/Game/BP/Gameplay/Grapple_BP.Grapple_BP_C|GetAttachedObject (stale Input|ActionEvents|InputActionRightFire _returnvalue_6)) "None" (Variables|/Game/BP/Gameplay/Grapple_BP.Grapple_BP_C|GetCollisionComponent (stale Input|ActionEvents|InputActionRightFire _returnvalue_6)) "None")
                                                (bind _returnvalue_18 (AddComponent|AddPhysicsConstraintComponent (stale Input|ActionEvents|InputActionRightFire _returnvalue_6) false))
                                                (Class|PhysicsConstraintComponent|SetConstrainedComponents _returnvalue_18 (Variables|/Game/BP/Gameplay/Grapple_BP.Grapple_BP_C|GetCollisionComponent (stale Input|ActionEvents|InputActionRightFire _returnvalue_6)) "None" (Variables|Default|GetCapsuleCollisionComponent) "None")
                                                (if true
                                                  (goto _label_12 Open)))))
                                          (:then_1
                                            (Utilities|IsValid _returnvalue_17
                                              (:Is%20Valid
                                                (Utilities|IsValid (Variables|/Game/BP/Gameplay/Grapple_BP.Grapple_BP_C|GetAttachedObject (stale Input|ActionEvents|InputActionRightFire _returnvalue_6))
                                                  (:Is%20Not%20Valid
                                                    (goto _label_12 Close))))))
                                          (:then_2
                                            (if (Utilities|ClassIsChildOf (Utilities|GetClass (Variables|/Game/BP/Gameplay/Grapple_BP.Grapple_BP_C|GetAttachedObjectActor (stale Input|ActionEvents|InputActionRightFire _returnvalue_6))) "/Game/BP/LevelAssets/RKT_Ball.RKT_Ball_C")
                                              (if (not (Utilities|ClassIsChildOf (Utilities|GetClass (Variables|/Game/BP/Gameplay/Grapple_BP.Grapple_BP_C|GetAttachedObjectActor (stale Input|ActionEvents|InputActionRightFire _returnvalue_6))) "/Game/BP/Gameplay/Grapple_BP.Grapple_BP_C"))
                                                (Utilities|FlowControl|Sequence
                                                  (:then_0
                                                    (bind _output_get (Variables|Default|SetAttachedObjRef_Alt (Variables|/Game/BP/Gameplay/Grapple_BP.Grapple_BP_C|GetAttachedObject (stale Input|ActionEvents|InputActionRightFire _returnvalue_6))))
                                                    (Collision|SetCollisionObjectType _output_get "ECC_GameTraceChannel1"))
                                                  (:then_1
                                                    (bind _output_get_2 (Variables|Default|SetBallIgnored_Alt true))))))))))))
                                (else
                                  ;;[1 1 1] Comment
                                  (if (Variables|/Game/BP/Gameplay/Grapple_BP.Grapple_BP_C|GetAttachedToStatic (stale Input|ActionEvents|InputActionRightFire _returnvalue_6))
                                    ;;[0 1 0.4565] Attached to Static Object
                                    (if true
                                      (if (not (Utilities|ClassIsChildOf (Utilities|GetClass (.HitComponent (Collision|BreakHitResult (stale _outhit_3)))) "RKTPawn_BP_C"))
                                        (Utilities|IsValid (Variables|/Game/BP/Gameplay/Grapple_BP.Grapple_BP_C|GetAttachedStatic (stale Input|ActionEvents|InputActionRightFire _returnvalue_6))
                                          (:Is%20Valid
                                            (if (not (Utilities|ClassIsChildOf (Utilities|GetClass (.HitComponent (Collision|BreakHitResult (stale _outhit_3)))) "/Script/Landscape.Landscape"))
                                              (Utilities|FlowControl|Sequence
                                                (:then_0
                                                  (Utilities|FlowControl|DoOnce false :!label _label_9
                                                    (:Completed
                                                      (bind _returnvalue_19 (AddComponent|AddPhysicsConstraintComponent (Variables|/Game/BP/Gameplay/Grapple_BP.Grapple_BP_C|GetAttachedStaticActor (stale Input|ActionEvents|InputActionRightFire _returnvalue_6)) false))
                                                      (Class|PhysicsConstraintComponent|SetConstrainedComponents _returnvalue_19 (Variables|/Game/BP/Gameplay/Grapple_BP.Grapple_BP_C|GetAttachedStatic (stale Input|ActionEvents|InputActionRightFire _returnvalue_6)) "None" (Variables|/Game/BP/Gameplay/Grapple_BP.Grapple_BP_C|GetAttachedStatic (stale Input|ActionEvents|InputActionRightFire _returnvalue_6)) "None")
                                                      (bind _returnvalue_20 (AddComponent|AddPhysicsConstraintComponent (stale Input|ActionEvents|InputActionRightFire _returnvalue_6) false))
                                                      (Class|PhysicsConstraintComponent|SetConstrainedComponents _returnvalue_20 (Variables|/Game/BP/Gameplay/Grapple_BP.Grapple_BP_C|GetCollisionComponent (stale Input|ActionEvents|InputActionRightFire _returnvalue_6)) "None" (Variables|Default|GetRocketMesh_Ref) "None")
                                                      (if true
                                                        (goto _label_13 Open)))))
                                                (:then_1
                                                  (Utilities|IsValid _returnvalue_19
                                                    (:Is%20Valid
                                                      (Utilities|IsValid (Variables|/Game/BP/Gameplay/Grapple_BP.Grapple_BP_C|GetAttachedStatic (stale Input|ActionEvents|InputActionRightFire _returnvalue_6))
                                                        (:Is%20Not%20Valid
                                                          (goto _label_13 Close)))))))))))))))))
                          (:then_1
                            ;;[1 1 1] Line Trace to detect hits along grapple route
                            (bind (_outhit_3 _returnvalue_21) (Collision|LineTraceByChannel _returnvalue_11 (Transformation|GetWorldLocation (Variables|/Game/BP/Gameplay/Grapple_BP.Grapple_BP_C|GetSphere (stale Input|ActionEvents|InputActionRightFire _returnvalue_6))) "TraceTypeQuery1" false (Utilities|Array|MakeArray (stale Input|ActionEvents|InputActionRightFire _returnvalue_6) (Variables|/Game/BP/Gameplay/Grapple_BP.Grapple_BP_C|GetAttachedObjectActor (stale Input|ActionEvents|InputActionRightFire _returnvalue_6)) (Variables|/Game/BP/Gameplay/Grapple_BP.Grapple_BP_C|GetAttachedStaticActor (stale Input|ActionEvents|InputActionRightFire _returnvalue_6))) "None"))
                            (if _returnvalue_21
                              (if (not (Variables|/Game/BP/Gameplay/Grapple_BP.Grapple_BP_C|GetAttachedToObject (stale Input|ActionEvents|InputActionRightFire _returnvalue_6)))
                                (Utilities|FlowControl|DoOnce false :!label _label_10
                                  (:Completed
                                    (Transformation|SetActorLocation (stale Input|ActionEvents|InputActionRightFire _returnvalue_6) (.ImpactPoint (Collision|BreakHitResult _outhit_3)) false false)
                                    (goto _label_7))))))))))
                  (:then_1
                    ;;[0 0 0] Conditional Destroy Actor Spaghetti
                    (Variables|Default|SetCableSlackLength (Math|Vector|VectorLength (- (Transformation|GetActorLocation (stale Input|ActionEvents|InputActionRightFire _returnvalue_6)) (Transformation|GetActorLocation))))
                    (if (Variables|/Game/BP/Gameplay/Grapple_BP.Grapple_BP_C|GetAttachedToObject (stale Input|ActionEvents|InputActionRightFire _returnvalue_6))
                      (if (> (Variables|Default|GetCableSlackLength) 2e+03)
                        (Utilities|IsValid (stale Input|ActionEvents|InputActionRightFire _returnvalue_6) :!label _label_11
                          (:Is%20Valid
                            _)
                          (:Is%20Not%20Valid
                            _))
                        (Actor|DestroyActor (stale Input|ActionEvents|InputActionRightFire _returnvalue_6))
                        (Utilities|FlowControl|Sequence
                          (:then_0
                            (goto _label_7 Close))
                          (:then_1
                            (Utilities|FlowControl|Gate true :!label _label_12
                              (:Exit
                                (Class|PhysicsConstraintComponent|BreakConstraint _returnvalue_17)
                                (Class|PhysicsConstraintComponent|BreakConstraint _returnvalue_18)
                                (Utilities|FlowControl|Sequence
                                  (:then_0
                                    (goto _label_8 Reset))
                                  (:then_1
                                    (goto _label_6))))))
                          (:then_2
                            (Utilities|FlowControl|Gate true :!label _label_13
                              (:Exit
                                (Class|PhysicsConstraintComponent|BreakConstraint _returnvalue_19)
                                (Class|PhysicsConstraintComponent|BreakConstraint _returnvalue_20)
                                (Utilities|FlowControl|Sequence
                                  (:then_0
                                    (goto _label_9 Reset))
                                  (:then_1
                                    (goto _label_6))))))
                          (:then_4
                            (Utilities|FlowControl|DoOnce false) ; enters at Reset
                          )
                          (:then_5
                            (if true
                              (goto _label_10 Reset)))))
                      (else
                        (Utilities|FlowControl|Delay 3.0)
                        (if (not (Variables|/Game/BP/Gameplay/Grapple_BP.Grapple_BP_C|GetAttachedToObject (stale Input|ActionEvents|InputActionRightFire _returnvalue_6)))
                          (goto _label_11))))))))))))))

(event EventBeginPlay
  ;[0 1 0.4287] BeginPlay - Set Static Mesh - Rocket Mesh Reference
  (Variables|Default|SetRocketMesh_Ref (Variables|Default|GetRocketMesh)))

(event Input|ActionEvents|InputActionFire
  (params (Key :type Key%20Structure :default "AnyKey"))
  (bind _returnvalue (Math|Rotator|MakeRotator 0.0 0.0 -9e+01))
  (bind _returnvalue_2 (Transformation|GetActorRotation))
  (bind _rocketmesh_ref (Variables|Default|GetRocketMesh_Ref))
  (bind _rocketmesh (Variables|Default|GetRocketMesh))
  (bind _rocketmesh_ref_2 (Variables|Default|GetRocketMesh_Ref))
  (bind _rocketmesh_ref_3 (Variables|Default|GetRocketMesh_Ref))
  (bind _rocketmesh_ref_4 (Variables|Default|GetRocketMesh_Ref))
  (bind _rocketmesh_ref_5 (Variables|Default|GetRocketMesh_Ref))
  (bind _rocketmesh_ref_6 (Variables|Default|GetRocketMesh_Ref))
  (bind _returnvalue_3 (Math|Rotator|CombineRotators _returnvalue_2 _returnvalue))
  (bind _returnvalue_4 (Transformation|GetSocketLocation _rocketmesh "RKT_L_Hook_Socket"))
  (bind _returnvalue_5 (+ _returnvalue_4 "0, 0, 0"))
  (:Pressed
    (Networking|SwitchHasAuthority
      (:Authority
        (Utilities|FlowControl|Sequence
          (:then_0
            (Utilities|FlowControl|DoOnce false :!label _label
              (:Completed
                (Utilities|FlowControl|Sequence
                  (:then_0
                    (bind _returnvalue_6 (Game|SpawnActorfromClass "/Game/BP/Gameplay/Grapple_BP.Grapple_BP_C" (Math|Transform|MakeTransform _returnvalue_5 _returnvalue_3) "AdjustIfPossibleButAlwaysSpawn" (Game|GetPlayerController 0) "0.000000,0.000000,0.000000" true false false)) ; Spawn Projectile
                    (bind _returnvalue_7 (Physics|GetPhysicsLinearVelocity (Variables|Default|GetCapsuleCollisionComponent) "None"))
                    (Physics|AddImpulse (Variables|/Game/BP/Gameplay/Grapple_BP.Grapple_BP_C|GetCollisionComponent _returnvalue_6) (+ (* _returnvalue_7 1.0) (Math|Vector|RotateVector "5000.000000, 0, 0" _returnvalue_3)) "None" true)
                    (Utilities|FlowControl|Gate true) ; enters at Open
                  )))))
          (:then_1
            ;[0 0 0] Conditional Destroy Actor Spaghetti
            (if (Variables|/Game/BP/Gameplay/Grapple_BP.Grapple_BP_C|GetAttachedToObject _returnvalue_6)
              (Utilities|IsValid _returnvalue_6 :!label _label_2
                (:Is%20Valid
                  _)
                (:Is%20Not%20Valid
                  _))
              (Actor|DestroyActor _returnvalue_6)
              (Utilities|FlowControl|Sequence
                (:then_0
                  (Utilities|FlowControl|Gate true) ; enters at Close
                )
                (:then_2
                  ;[0 1 0.4565] Attached to Static Object
                  (Utilities|FlowControl|Gate true
                    (:Exit
                      (Class|PhysicsConstraintComponent|BreakConstraint (stale EventTick _returnvalue_13))
                      (Class|PhysicsConstraintComponent|BreakConstraint (stale EventTick _returnvalue_14))
                      (Utilities|FlowControl|Sequence
                        (:then_0
                          (Utilities|FlowControl|DoOnce false) ; enters at Reset
                        )
                        (:then_1
                          ;[1 0.004134 0] Fixes most constraint physics bugs after break
                          (Class|PrimitiveComponent|SetAllPhysicsLinearVelocity _rocketmesh_ref_2 "0, 0, 0" false)
                          (Physics|SetSimulatePhysics _rocketmesh_ref_2 false)
                          (Physics|SetSimulatePhysics _rocketmesh_ref_2 true))))))
                (:then_4
                  (goto _label Reset))
                (:then_5
                  ;[0.6243 0.7252 1] Line Trace to detect hits along grapple route
                  ;;[1 1 1] Connects from Destroy Spaghetti
                  (if true
                    (Utilities|FlowControl|DoOnce false) ; enters at Reset
                  ))
                (:then_6
                  (Variables|Default|SetGrappleReleased true)
                  (if (Variables|Default|GetGrappleReleased)
                    (Utilities|FlowControl|Sequence
                      (:then_0
                        ;[1 0.004134 0] Fixes most constraint physics bugs after break
                        (Class|PrimitiveComponent|SetAllPhysicsLinearVelocity _rocketmesh_ref_3 "0, 0, 0" false)
                        (Physics|SetSimulatePhysics _rocketmesh_ref_3 false)
                        (Physics|SetSimulatePhysics _rocketmesh_ref_3 true)))))
                (:then_7
                  (Class|PrimitiveComponent|SetAngularDamping _rocketmesh_ref_5 0.0)
                  (Class|PrimitiveComponent|SetLinearDamping _rocketmesh_ref_5 0.01)
                  (Class|PrimitiveComponent|SetAngularDamping (Variables|/Game/BP/Gameplay/Grapple_BP.Grapple_BP_C|GetAttachedObject _returnvalue_6) 0.0)
                  (Class|PrimitiveComponent|SetLinearDamping (Variables|/Game/BP/Gameplay/Grapple_BP.Grapple_BP_C|GetAttachedObject _returnvalue_6) 0.01)))
              (else
                (Utilities|FlowControl|Delay 1.0)
                (if (not (Variables|/Game/BP/Gameplay/Grapple_BP.Grapple_BP_C|GetAttachedToObject _returnvalue_6))
                  (goto _label_2))))))))))

(event Input|ActionEvents|InputActionRightFire
  (params (Key :type Key%20Structure :default "AnyKey"))
  (bind _returnvalue (Math|Rotator|MakeRotator 0.0 0.0 9e+01))
  (bind _returnvalue_2 (Transformation|GetActorRotation))
  (bind _rocketmesh (Variables|Default|GetRocketMesh))
  (bind _rocketmesh_ref (Variables|Default|GetRocketMesh_Ref))
  (bind _returnvalue_3 (Math|Rotator|CombineRotators _returnvalue_2 _returnvalue))
  (bind _returnvalue_4 (Transformation|GetSocketLocation _rocketmesh_ref "RKT_R_Hook_Socket"))
  (bind _returnvalue_5 (+ _returnvalue_4 "0, 0, 0"))
  ;[0 0.01606 1] Alt Fire
  (:Pressed
    (Utilities|FlowControl|Sequence
      (:then_0
        (Utilities|FlowControl|DoOnce false :!label _label
          (:Completed
            (Utilities|FlowControl|Sequence
              (:then_0
                (bind _returnvalue_6 (Game|SpawnActorfromClass "/Game/BP/Gameplay/Grapple_BP.Grapple_BP_C" (Math|Transform|MakeTransform _returnvalue_5 _returnvalue_3) "AdjustIfPossibleButAlwaysSpawn" 0 "0.000000,0.000000,0.000000" true false false)) ; Spawn Projectile
                (bind _returnvalue_7 (Physics|GetPhysicsLinearVelocity (Variables|Default|GetCapsuleCollisionComponent) "None"))
                (Physics|AddImpulse (Variables|/Game/BP/Gameplay/Grapple_BP.Grapple_BP_C|GetCollisionComponent _returnvalue_6) (+ (* _returnvalue_7 1.0) (Math|Vector|RotateVector "5000.000000, 0, 0" _returnvalue_3)) "None" true)
                (Utilities|FlowControl|Gate true) ; enters at Open
              )))))
      (:then_1
        ;;[0 0 0] Conditional Destroy Actor Spaghetti
        (if (Variables|/Game/BP/Gameplay/Grapple_BP.Grapple_BP_C|GetAttachedToObject _returnvalue_6)
          (Utilities|IsValid _returnvalue_6 :!label _label_2
            (:Is%20Valid
              _)
            (:Is%20Not%20Valid
              _))
          (Actor|DestroyActor _returnvalue_6)
          (Utilities|FlowControl|Sequence
            (:then_0
              (Utilities|FlowControl|Gate true) ; enters at Close
            )
            (:then_1
              ;;[1 0.9702 0] Attached to Dynamic Object
              (Utilities|FlowControl|Gate true
                (:Exit
                  (Class|PhysicsConstraintComponent|BreakConstraint (stale EventTick _returnvalue_17))
                  (Class|PhysicsConstraintComponent|BreakConstraint (stale EventTick _returnvalue_18))
                  (Utilities|FlowControl|Sequence
                    (:then_0
                      (Utilities|FlowControl|DoOnce false) ; enters at Reset
                    )
                    (:then_1
                      ;;[1 0.004134 0] Fixes most constraint physics bugs after break
                      (Class|PrimitiveComponent|SetAllPhysicsLinearVelocity _rocketmesh "0, 0, 0" false :!label _label_3)
                      (Physics|SetSimulatePhysics _rocketmesh false)
                      (Physics|SetSimulatePhysics _rocketmesh true))))))
            (:then_2
              ;;[0 1 0.4565] Attached to Static Object
              (Utilities|FlowControl|Gate true
                (:Exit
                  (Class|PhysicsConstraintComponent|BreakConstraint (stale EventTick _returnvalue_19))
                  (Class|PhysicsConstraintComponent|BreakConstraint (stale EventTick _returnvalue_20))
                  (Utilities|FlowControl|Sequence
                    (:then_0
                      (Utilities|FlowControl|DoOnce false) ; enters at Reset
                    )
                    (:then_1
                      (goto _label_3))))))
            (:then_4
              (goto _label Reset))
            (:then_5
              ;;[1 1 1] Line Trace to detect hits along grapple route
              (if true
                (Utilities|FlowControl|DoOnce false) ; enters at Reset
              )))
          (else
            (Utilities|FlowControl|Delay 3.0)
            (if (not (Variables|/Game/BP/Gameplay/Grapple_BP.Grapple_BP_C|GetAttachedToObject _returnvalue_6))
              (goto _label_2))))))))

(fn ConstructionScript)